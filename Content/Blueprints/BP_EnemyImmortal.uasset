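; BP_EnemyImmortal is an enemy that kills the player on contact and patrols along a spline.
; Each tick it teleports to the constant-velocity spline point for its elapsed time, which counts up or down and flips direction past either end for a ping-pong path.
; A capsule hit on BP_Player calls Die on the player and stops the enemy's movement.
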(event OnComponentHit(CapsuleComponent)
  (params (HitComponent :type Primitive%20Component%20Object%20Reference) (OtherActor :type Actor%20Object%20Reference) (OtherComp :type Primitive%20Component%20Object%20Reference) (NormalImpulse :type Vector :default "0, 0, 0") (Hit :type Hit%20Result%20Structure%20%28by%20ref%29))
  ;[1 1 1] Collision with player
  (bind _asbp_player (Utilities|Casting|CastToBP_Player OtherActor))
  (Default|Die _asbp_player)
  (Variables|Default|SetMove false))

(event EventTick
  (params (DeltaSeconds :type Float%20%28single-precision%29))
  (if (and (Variables|Default|GetMove) (Utilities|IsValid (Variables|Default|GetPatrolSpline)))
    (Transformation|SetActorLocation (Spline|GetLocationatTime (Variables|/Game/Blueprints/BP_PatrolSpline.BP_PatrolSpline_C|GetSpline (Variables|Default|GetPatrolSpline)) (Variables|Default|GetElapsedTime) "World" true) false true)
    (bind _output_get (Variables|Default|SetElapsedTime (Math|Float|SelectFloat (+ (Variables|Default|GetElapsedTime) DeltaSeconds) (- (Variables|Default|GetElapsedTime) DeltaSeconds) (Variables|Default|GetForward))))
    (if (or (< _output_get 0.0) (> _output_get (Variables|/Script/Engine.SplineComponent|GetDuration (Variables|/Game/Blueprints/BP_PatrolSpline.BP_PatrolSpline_C|GetSpline (Variables|Default|GetPatrolSpline)))))
      (Variables|Default|SetForward (not (Variables|Default|GetForward))))))

(fn ConstructionScript)