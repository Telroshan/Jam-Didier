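; BP_Enemy is an enemy that turns to face the player, fires projectiles at them and destroys itself when its capsule hits BP_Player.
; On BeginPlay it caches the player pawn and starts Shoot, which re-triggers itself after each ReloadDelay.
; Each shot spawns a BP_EnemyProjectile at ShootPoint and sets its Direction toward the player's current position.
; Tick rotates the enemy toward the player using only the look-at yaw.
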(event OnComponentHit(CapsuleComponent)
  (params (HitComponent :type Primitive%20Component%20Object%20Reference) (OtherActor :type Actor%20Object%20Reference) (OtherComp :type Primitive%20Component%20Object%20Reference) (NormalImpulse :type Vector :default "0, 0, 0") (Hit :type Hit%20Result%20Structure%20%28by%20ref%29))
  ;[1 1 1] Collision with player
  (Utilities|Casting|CastToBP_Player OtherActor)
  (Actor|DestroyActor))

(event Custom|Shoot
  (bind _shootpoint (Variables|Default|GetShootPoint))
  (bind _returnvalue (Transformation|GetWorldLocation _shootpoint))
  ;[1 1 1] Shoot at player
  (bind _returnvalue_2 (Game|SpawnActorfromClass "/Game/Blueprints/BP_EnemyProjectile.BP_EnemyProjectile_C" (Math|Transform|MakeTransform _returnvalue "0, 0, 0" "1,1,1") "Undefined" 0 0))
  (Variables|/Game/Blueprints/BP_EnemyProjectile.BP_EnemyProjectile_C|SetDirection _returnvalue_2 (Math|Vector|Normalize (- (Transformation|GetActorLocation (Variables|Default|GetPlayer)) _returnvalue)))
  (Utilities|FlowControl|Delay (Variables|Default|GetReloadDelay))
  (CallFunction|Shoot))

(event EventBeginPlay
  ;[1 1 1] Shoot at player
  (bind _asbp_player (Utilities|Casting|CastToBP_Player (Game|Player|GetPlayerPawn 0)))
  (Variables|Default|SetPlayer _asbp_player)
  (CallFunction|Shoot))

(event EventTick
  (params (DeltaSeconds :type Float%20%28single-precision%29))
  ;[1 1 1] Look at player
  (Transformation|SetActorRotation (Math|Rotator|MakeRotator 0.0 0.0 (.yaw (Math|Rotator|FindLookatRotation (Transformation|GetActorLocation) (Transformation|GetActorLocation (Variables|Default|GetPlayer)))))))

(fn ConstructionScript)