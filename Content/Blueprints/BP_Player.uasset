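; Player pawn for a slingshot-style physics ball that dashes to kill every BP_Enemy.
; Holding Aim slows time and shows an arrow and aim widget; releasing restores time and launches the Sphere.
; GetBallDirection converts mouse drag into a camera-yaw-relative vector, clamped to MaxImpulse, driving both arrow and launch velocity.
; Die shows game over, OnKill counts toward the win screen; once play ends, Tick hides aiming and zeroes velocity.
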(event Custom|Die
  ;[1 1 1] Die
  (if (Variables|Default|GetPlaying)
    (Variables|Default|SetPlaying false)
    (bind _returnvalue (UserInterface|CreateWidget "/Game/Blueprints/WBP_GameOver.WBP_GameOver_C"))
    (UserInterface|Viewport|AddtoViewport _returnvalue 0)
    (Audio|PlaySound2D "/Game/Audio/fuck2.fuck2" 1.0 1.0 0.0 0 0)))

(event Custom|OnKill
  ;[1 1 1] OnKill
  (if (Variables|Default|GetPlaying)
    (bind _result (Math|Integer|IncrementInt (Variables|Default|GetEnemiesKilledCount))
      (:%20%20
        (if (>= _result (Variables|Default|GetEnemiesCount))
          (Variables|Default|SetPlaying false)
          (bind _returnvalue (UserInterface|CreateWidget "/Game/Blueprints/WBP_Win.WBP_Win_C"))
          (UserInterface|Viewport|AddtoViewport _returnvalue 0)
          (Utilities|FlowControl|Delay 1.0)
          (Audio|PlaySound2D "/Game/Audio/yeah2_Cue.yeah2_Cue" 1.0 1.0 0.0 0 0))))))

(event EventBeginPlay
  (bind _returnvalue (Game|GetPlayerController 0))
  ;[1 1 1] Init
  (Variables|/Script/Engine.PlayerController|SetbShowMouseCursor _returnvalue true)
  (bind _returnvalue_2 (UserInterface|CreateWidget "/Game/Blueprints/WBP_AimUI.WBP_AimUI_C" _returnvalue))
  (bind _output_get (Variables|Default|SetAimWidget _returnvalue_2))
  (UserInterface|Viewport|AddtoViewport _output_get 0)
  (Widget|SetVisibility (Variables|Default|GetAimWidget) "Hidden")
  (bind _outactors (Actor|GetAllActorsOfClass "/Game/Blueprints/BP_Enemy.BP_Enemy_C"))
  (Variables|Default|SetEnemiesCount (Utilities|Array|Length _outactors))
  (Variables|Default|SetEnemiesKilledCount 0))

(event EventTick
  (params (DeltaSeconds :type Float%20%28single-precision%29))
  ;[1 1 1] Aim arrow + UI update
  (if (Variables|Default|GetPlaying)
    (Utilities|FlowControl|Sequence
      (:then_0
        (bind _newparam (CallFunction|GetBallDirection))
        (Transformation|SetWorldRotation (Variables|Default|GetAimArrow) (Math|Rotator|FindLookatRotation (Math|Vector|VectorZero) _newparam) false false))
      (:then_1
        (bind _returnvalue (Class|WidgetLayoutLibrary|GetMousePositiononViewport))
        (Variables|/Game/Blueprints/WBP_AimUI.WBP_AimUI_C|SetAimPoint (Variables|Default|GetAimWidget) (* (- (Variables|Default|GetAimPoint) _returnvalue) -1.0))))
    (else
      (Widget|SetVisibility (Variables|Default|GetAimWidget) "Hidden")
      (Rendering|SetVisibility (Variables|Default|GetAimArrow) false false)
      (Physics|SetPhysicsLinearVelocity (Variables|Default|GetSphere) "0, 0, 0" false "None"))))

(event Input|ActionEvents|InputActionAim
  (params (Key :type Key%20Structure :default "None"))
  (bind _aimwidget (Variables|Default|GetAimWidget))
  (:Pressed
    (if (Variables|Default|GetPlaying)
      ;[1 1 1] Aim
      (bind _returnvalue (Class|WidgetLayoutLibrary|GetMousePositiononViewport))
      (Variables|Default|SetAimPoint _returnvalue)
      (Utilities|Time|SetGlobalTimeDilation (Variables|Default|GetTimeSlowFactor))
      (Rendering|SetVisibility (Variables|Default|GetAimArrow) true false)
      (Class|UserWidget|SetPositioninViewport _aimwidget (Variables|Default|GetAimPoint) false)
      (Variables|/Game/Blueprints/WBP_AimUI.WBP_AimUI_C|SetAimPoint _aimwidget (Variables|Default|GetAimPoint))
      (Widget|SetVisibility _aimwidget "Visible")
      (Audio|PlaySound2D "/Game/Audio/za-warudo-sound-effect2_Cue.za-warudo-sound-effect2_Cue" 1.0 1.0 0.0 0 0)
      (Audio|PlaySound2D "/Game/Audio/aim.aim" 1.0 1.0 0.0 0 0)))
  (:Released
    (if (Variables|Default|GetPlaying)
      ;[1 1 1] Shoot
      (bind _newparam (CallFunction|GetBallDirection))
      (Physics|SetPhysicsLinearVelocity (Variables|Default|GetSphere) (* _newparam (Variables|Default|GetDashImpulse)) false "None")
      (Utilities|Time|SetGlobalTimeDilation 1.0)
      (Rendering|SetVisibility (Variables|Default|GetAimArrow) false false)
      (Widget|SetVisibility (Variables|Default|GetAimWidget) "Hidden")
      (Audio|PlaySound2D "/Game/Audio/release.release" 1.0 1.0 0.0 0 0))))

(fn ConstructionScript)

(fn GetBallDirection
  (bind _maximpulse (Variables|Default|GetMaxImpulse))
  (bind _returnvalue (Class|WidgetLayoutLibrary|GetMousePositiononViewport))
  (return (Math|Vector|SelectVector (* (Math|Vector|Normalize (Math|Vector|RotateVector (Math|Conversions|ToVector(Vector2D) (- (Variables|Default|GetAimPoint) _returnvalue)) (Math|Rotator|MakeRotator 0.0 0.0 (+ (.yaw (Transformation|GetWorldRotation (Variables|Default|GetSpringArm))) 9e+01)))) _maximpulse) (Math|Vector|RotateVector (Math|Conversions|ToVector(Vector2D) (- (Variables|Default|GetAimPoint) _returnvalue)) (Math|Rotator|MakeRotator 0.0 0.0 (+ (.yaw (Transformation|GetWorldRotation (Variables|Default|GetSpringArm))) 9e+01))) (> (Math|Vector|VectorLength (Math|Vector|RotateVector (Math|Conversions|ToVector(Vector2D) (- (Variables|Default|GetAimPoint) _returnvalue)) (Math|Rotator|MakeRotator 0.0 0.0 (+ (.yaw (Transformation|GetWorldRotation (Variables|Default|GetSpringArm))) 9e+01)))) _maximpulse))))